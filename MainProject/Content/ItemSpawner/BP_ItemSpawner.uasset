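; BP_ItemSpawner is a spawner actor that creates a random item at its own location when play begins and on respawn.
; SpawnItem picks a class from the ItemsToSpawn array and spawns it with the spawner's transform at unit scale, as its owner.
; The Respawn event calls SpawnItem again after a fixed delay.
; The random index range includes the array length, so it can land out of bounds.
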(event `self.ReceiveBeginPlay`
  (`self.SpawnItem`))

(event `/Game/Blueprints/Interact.Respawn`
  (`KismetSystemLibrary.Delay` 5.0)
  (`self.SpawnItem`))

(fn `SpawnItem`
  (bind _itemstospawn (`self.ItemsToSpawn`))
  (`|SpawnActorFromClass` (`|GetArrayItem` _itemstospawn (`KismetMathLibrary.RandomIntegerInRange` 0 (`KismetArrayLibrary.Array_Length` _itemstospawn))) (`KismetMathLibrary.MakeTransform` (`self.K2_GetActorLocation`) (`self.K2_GetActorRotation`)) "AdjustIfPossibleButAlwaysSpawn" "OverrideRootScale" self (struct) null))

(fn `UserConstructionScript`)