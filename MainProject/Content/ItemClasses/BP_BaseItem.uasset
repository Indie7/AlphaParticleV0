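; BP_BaseItem is a base actor for pickup items that go into the player's inventory.
; Interact sends RespawnMessage to its owner, destroys the actor and adds its ItemData, stamped with its own class, to the player's Inventory.
; LookedAt replaces the player's current LookingAtWidget with a new LookingAtItem widget, and OnUsed is an empty event.
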(event `/Game/Blueprints/Interact.Interact`
  (params (Player :type "/Game/Blueprints/Player Object Reference"))
  (message `/Game/Blueprints/Interact.Respawn` (`self.GetOwner`))
  (`self.K2_DestroyActor`)
  (bind _structout (setmembers `/Game/InventorySystem/Blueprints/Structures/S_InventoryStructure` :`StructRef` (`self.ItemData`) :`ActorClass` (`GameplayStatics.GetObjectClass` self)))
  (`KismetArrayLibrary.Array_Add` (`/Game/Blueprints/Player.Inventory` Player) _structout))

(event `Event On Used`)

(fn `LookedAt`
  (params (Player :type "/Game/Blueprints/Player Object Reference"))
  (returns (Triggered :type Boolean))
  (bind _lookingatwidget (`/Game/Blueprints/Player.LookingAtWidget` Player))
  (`/Engine/EditorBlueprintResources/StandardMacros.IsValid` _lookingatwidget
    (:`Is Valid`
      (`Widget.RemoveFromParent` _lookingatwidget))
    (:`Is Not Valid`
      _))
  (bind _returnvalue (`|CreateWidget` "/Game/Blueprints/LookingAtItem.LookingAtItem_C"))
  (bind _output_get (set `/Game/Blueprints/Player.LookingAtWidget` _returnvalue Player))
  (`UserWidget.AddToViewport` _output_get 0)
  (return true))

(fn `UserConstructionScript`)